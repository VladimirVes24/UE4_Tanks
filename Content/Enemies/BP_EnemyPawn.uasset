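; Enemy pawn that takes damage and explodes when killed.
; AnyDamage subtracts from Health, then sets IsDead and destroys the actor once Health reaches zero or below.
; On Destroyed, it spawns oversized explosion, fire and smoke emitters at its location, so the effects play on any destruction, not just death by damage.
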(event `self.ReceiveAnyDamage`
  (params (Damage :type "Float (single-precision)") (DamageType :type "DamageType Object Reference") (InstigatedBy :type "Controller Object Reference") (DamageCauser :type "Actor Object Reference"))
  (set `self.Health` (- (`self.Health`) Damage))
  (if (<= (`self.Health`) 0.0)
    (set `self.IsDead` true)
    (`self.K2_DestroyActor`)))

(event `self.ReceiveDestroyed`
  (bind _returnvalue (`self.K2_GetActorLocation`))
  (`GameplayStatics.SpawnEmitterAtLocation` "/Game/CSC/Demo/Particles/P_Explosion.P_Explosion" _returnvalue (struct) (20.0 20.0 20.0))
  (`GameplayStatics.SpawnEmitterAtLocation` "/Game/Effects/P_Fire.P_Fire" _returnvalue (struct) (20.0 20.0 20.0))
  (`GameplayStatics.SpawnEmitterAtLocation` "/Game/Effects/P_Smoke.P_Smoke" _returnvalue (struct) (20.0 20.0 20.0)))

(fn `UserConstructionScript`)