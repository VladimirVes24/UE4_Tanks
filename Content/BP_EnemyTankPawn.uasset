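; Enemy tank pawn Blueprint whose event graph is effectively inert: all events are empty and the HUD, pause and game-over blocks are disconnected.
; The unwired blocks look like player-tank logic, updating health, ammo and fire-rate widgets and showing menus through TanksHUD.
; LowerHealth subtracts a fixed amount of HP and destroys the actor at zero, but only an unwired block calls it here.
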(event `self.ReceiveAnyDamage`
  (params (Damage :type "Float (single-precision)") (DamageType :type "DamageType Object Reference") (InstigatedBy :type "Controller Object Reference") (DamageCauser :type "Actor Object Reference")))

(event `self.ReceiveActorBeginOverlap`
  (params (OtherActor :type "Actor Object Reference")))

(event `Key|K`
  (params (Key :type "Key Structure"))
  ;[1 1 1] LowerHP
)

(event `self.ReceiveDestroyed`
  ;[1 1 1] GameOver
)

(event `Key|P`
  (params (Key :type "Key Structure"))
  ;[1 1 1] Pause
)

(event `self.ReceiveBeginPlay`
  ;[1 1 1] Begin Play Statuses Update
)

(event `self.ReceiveTick`
  (params (DeltaSeconds :type "Float (single-precision)"))
  ;[1 1 1] Tick
)

(event `self.ReceiveHit`
  (params (MyComp :type "PrimitiveComponent Object Reference") (Other :type "Actor Object Reference") (OtherComp :type "PrimitiveComponent Object Reference") (bSelfMoved :type Boolean) (HitLocation :type "Vector Structure") (HitNormal :type "Vector Structure") (NormalImpulse :type "Vector Structure") (Hit :type "HitResult Structure (by ref)")))

(fn `Lower Health`
  (returns (IsDestroyed :type Boolean))
  (bind _output_get (set `self.HealthPointsCurrent` (- (`self.HealthPointsCurrent`) 25.0)))
  (if (<= _output_get 0.0)
    (`self.K2_DestroyActor`)
    (return true)))

(fn `UserConstructionScript`)